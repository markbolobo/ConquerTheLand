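; Demo actor for the overview that animates a tagged BP_Mesh_Border at runtime and tests helper actors against its area.
; BeginPlay caches the border and its tagged BP_Helper actors.
; Tick oscillates border width with a sine, eases corner roundness, refreshes and rotates it, while Delay-driven FlipFlops periodically toggle rounded corners and the roundness target.
; Each tick also sets every helper's active state by whether it lies inside the border.
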(event EventBeginPlay
  (bind _outactors (Actor|GetAllActorsOfClasswithTag "/Game/MapBorderCollection/Blueprints/BP_Mesh_Border.BP_Mesh_Border_C" "MeshBorder"))
  (Variables|Default|SetMeshBorder (Utilities|Array|Get(acopy) _outactors))
  (bind _outactors_2 (Actor|GetAllActorsOfClasswithTag "/Game/MapBorderCollection/Overview/Blueprints/Helper/BP_Helper.BP_Helper_C" "MeshHelper"))
  (Variables|Default|SetHelpers _outactors_2))

(event EventTick
  (params (DeltaSeconds :type Float%20%28single-precision%29))
  (bind _meshborder (Variables|Default|GetMeshBorder))
  (Utilities|IsValid (Variables|Default|GetMeshBorder)
    (:Is%20Valid
      (Variables|Default|SetDeltaTIme DeltaSeconds)
      (Variables|Default|SetTime (+ (Variables|Default|GetDeltaTIme) (Variables|Default|GetTime)))
      (Utilities|FlowControl|Sequence
        (:then_0
          (Variables|/Game/MapBorderCollection/Blueprints/BP_Mesh_Border.BP_Mesh_Border_C|SetBorderSIze (Variables|Default|GetMeshBorder) (Math|Vector2D|MakeVector2D (+ (- (* (Math|Trig|Sin(Radians) (Variables|Default|GetTime)) 1e+03) 3e+02) (.Y (Math|Vector2D|BreakVector2D (Variables|/Game/MapBorderCollection/Blueprints/BP_Mesh_Border.BP_Mesh_Border_C|GetBorderSIze (Variables|Default|GetMeshBorder))))) (.Y (Math|Vector2D|BreakVector2D (Variables|/Game/MapBorderCollection/Blueprints/BP_Mesh_Border.BP_Mesh_Border_C|GetBorderSIze (Variables|Default|GetMeshBorder))))))
          (Variables|/Game/MapBorderCollection/Blueprints/BP_Mesh_Border.BP_Mesh_Border_C|SetCornerRoundness (Variables|Default|GetMeshBorder) (Math|Interpolation|FInterpTo (Variables|/Game/MapBorderCollection/Blueprints/BP_Mesh_Border.BP_Mesh_Border_C|GetCornerRoundness (Variables|Default|GetMeshBorder)) (Variables|Default|GetCornerRoundnessTarget) (Variables|Default|GetDeltaTIme) 1.0))
          (Default|UpdateBorderinRuntime (Variables|Default|GetMeshBorder) false)
          (Transformation|AddActorLocalRotation (Variables|Default|GetMeshBorder) "0,1.000000, 0" false false)
          (Utilities|FlowControl|Sequence
            (:then_0
              (Utilities|FlowControl|Delay 2.0)
              (Utilities|FlowControl|FlipFlop
                (:A
                  (Variables|/Game/MapBorderCollection/Blueprints/BP_Mesh_Border.BP_Mesh_Border_C|SetRoundedCorners _meshborder false))
                (:B
                  (Variables|/Game/MapBorderCollection/Blueprints/BP_Mesh_Border.BP_Mesh_Border_C|SetRoundedCorners _meshborder true))))
            (:then_1
              (Utilities|FlowControl|Delay 1.7)
              (Utilities|FlowControl|FlipFlop
                (:A
                  (Variables|Default|SetCornerRoundnessTarget 2e+03))
                (:B
                  (Variables|Default|SetCornerRoundnessTarget 3e+02))))))
        (:then_1
          (for _array_element (Variables|Default|GetHelpers)
            (bind _success (Default|CheckifPointLiesInsideArea (Variables|Default|GetMeshBorder) (Math|Conversions|ToVector2D(Vector) (Transformation|GetActorLocation _array_element))))
            (Default|SetNewActiveState _array_element _success)))))))

(fn ConstructionScript)