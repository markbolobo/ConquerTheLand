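; RTS-style player controller for Conquer The Land that handles drag-box unit selection, move orders and hover cursors.
; Left-drag draws a HUD box; releasing without Shift clears the selection, projects the corners onto the land and runs two opposing box sweeps to select pawns.
; Right-click sends selected actors to the cursor location with growing acceptance radii and spawns click FX.
; Older HUD marquee press/release logic is left unconnected.
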(event Input|EnhancedActionEvents|EnhancedInputActionIA_RightMouseClick
  (params (ActionValue :type Boolean) (ElapsedSeconds :type Float%20%28double-precision%29) (TriggeredSeconds :type Float%20%28double-precision%29) (InputAction :type Input%20Action%20Object%20Reference :default "/Game/ConquerTheLand/Input/Actions/IA_RightMouseClick.IA_RightMouseClick"))
  (:Started
    (CallFunction|SelectActorMoveto)))

(event EventBeginPlay
  (bind _returnvalue (PlayerController|LocalPlayerSubsystems|GetEnhancedInputLocalPlayerSubsystem))
  (Input|SetInputModeGameandUI self 0 "LockAlways" false false)
  (Utilities|IsValid _returnvalue
    (:Is%20Valid
      (Input|AddMappingContext _returnvalue "/Game/ConquerTheLand/Input/IMC_CTLBase.IMC_CTLBase" 0 "(bIgnoreAllPressedKeysUntilRelease=True,bForceImmediately=False)"))))

(event EventTick
  (params (DeltaSeconds :type Float%20%28single-precision%29))
  (if (Variables|Default|GetmLeftMousePressed)
    (Class|BPIHUDBase|MarqueeHeld(Message) (HUD|GetHUD))))

(event EventRegisterSelectActor
  (params (SelectedActor :type Actor%20Object%20Reference))
  (Utilities|Array|Add (Variables|Default|GetmSelected%20Actor) SelectedActor))

(event EventOnHover
  (params (Enemy :type Boolean))
  (if (> (Utilities|Array|Length (Variables|Default|GetmSelected%20Actor)) 0)
    (Variables|Default|SetCurrentMouseCursor (select Enemy "Crosshairs" "Hand"))))

(event EventClearHover
  (Variables|Default|SetCurrentMouseCursor "Default"))

(fn ConstructionScript)

(fn SelectActorMoveto
  (bind _hitresult (Game|Player|GetHitResultUnderCursorbyChannel "TraceTypeQuery1" true))
  (bind _location (Collision|BreakHitResult _hitresult))
  (if (> (Utilities|Array|Length (Variables|Default|GetmSelected%20Actor)) 0)
    (for (_array_element _array_index) (Variables|Default|GetmSelected%20Actor)
      (Class|BPISTLCharacter|MovetoDestination(Message) _array_element _location (Math|Conversions|ToFloat(Integer) (* (+ _array_index 1) 100))))
    (Niagara|SpawnSystematLocation "/Game/Cursor/FX_Cursor.FX_Cursor" _location)))

(fn SelectDrawActor
  (bind (_locationx _locationy) (Game|Player|GetMousePosition))
  (bind _mstarsavepos (Variables|Default|GetmStarSavePos))
  (LocalVariables|SetaTempEndSavePos (Math|Vector2D|MakeVector2D _locationx _locationy))
  (if (> (Math|Vector|Distance2D(Vector) (LocalVariables|GetaTempEndSavePos) (Variables|Default|GetmStarSavePos)) 1.0)
    (Utilities|FlowControl|Sequence
      (:then_0
        (LocalVariables|SetaTempP1 (CallFunction|ScreentoLandMapping (Math|Vector2D|MakeVector2D (Math|Float|Min(Float) (.x _mstarsavepos) (.x (LocalVariables|GetaTempEndSavePos))) (Math|Float|Min(Float) (.y _mstarsavepos) (.y (LocalVariables|GetaTempEndSavePos))))))
        (LocalVariables|SetaTempP2 (CallFunction|ScreentoLandMapping (Math|Vector2D|MakeVector2D (Math|Float|Max(Float) (.x _mstarsavepos) (.x (LocalVariables|GetaTempEndSavePos))) (Math|Float|Min(Float) (.y _mstarsavepos) (.y (LocalVariables|GetaTempEndSavePos))))))
        (LocalVariables|SetaTempQ1 (CallFunction|ScreentoLandMapping (Math|Vector2D|MakeVector2D (Math|Float|Min(Float) (.x _mstarsavepos) (.x (LocalVariables|GetaTempEndSavePos))) (Math|Float|Max(Float) (.y _mstarsavepos) (.y (LocalVariables|GetaTempEndSavePos))))))
        (LocalVariables|SetaTempQ2 (CallFunction|ScreentoLandMapping (Math|Vector2D|MakeVector2D (Math|Float|Max(Float) (.x _mstarsavepos) (.x (LocalVariables|GetaTempEndSavePos))) (Math|Float|Max(Float) (.y _mstarsavepos) (.y (LocalVariables|GetaTempEndSavePos))))))
        (LocalVariables|SetaTempP1Q1%20half (Math|Vector|Lerp(Vector) (LocalVariables|GetaTempP1) (LocalVariables|GetaTempQ1) 0.5))
        (LocalVariables|SetaTempP1Q1%20Dis (Math|Vector|Distance(Vector) (LocalVariables|GetaTempP1) (LocalVariables|GetaTempQ1)))
        (LocalVariables|SetaTempP1Q1%20Rot (Math|Rotator|FindLookatRotation (LocalVariables|GetaTempP1) (LocalVariables|GetaTempQ1)))
        (LocalVariables|SetaTempHalf%20Box (Math|Vector|MakeVector (* (Math|Float|Min(Float) (LocalVariables|GetaTempP1Q1%20Dis) (Math|Vector|Distance(Vector) (LocalVariables|GetaTempP2) (LocalVariables|GetaTempQ2))) 0.5) 1e+01 4e+02))
        (LocalVariables|SetaTempEndPoint (+ (LocalVariables|GetaTempP1Q1%20half) (- (LocalVariables|GetaTempQ2) (LocalVariables|GetaTempQ1)))))
      (:then_1
        (bind (_outhits _returnvalue) (Class|KismetSystemLibrary|BoxTraceMultiforObjects (LocalVariables|GetaTempP1Q1%20half) (LocalVariables|GetaTempEndPoint) (LocalVariables|GetaTempHalf%20Box) (LocalVariables|GetaTempP1Q1%20Rot) (Utilities|Array|MakeArray "ObjectTypeQuery3") false 0 "None" true))
        (if _returnvalue
          (for _array_element _outhits
            (Utilities|Array|AddUnique (LocalVariables|GetaTempAllCharacters) (.HitActor (Collision|BreakHitResult _array_element)))))
        (bind (_outhits_2 _returnvalue_2) (Class|KismetSystemLibrary|BoxTraceMultiforObjects (Math|Vector|Lerp(Vector) (LocalVariables|GetaTempP2) (LocalVariables|GetaTempQ2) 0.5) (- (Math|Vector|Lerp(Vector) (LocalVariables|GetaTempP2) (LocalVariables|GetaTempQ2) 0.5) (- (LocalVariables|GetaTempQ2) (LocalVariables|GetaTempQ1))) (LocalVariables|GetaTempHalf%20Box) (Math|Rotator|FindLookatRotation (LocalVariables|GetaTempP2) (LocalVariables|GetaTempQ2)) (Utilities|Array|MakeArray "ObjectTypeQuery3") false 0 "None" true))
        (if _returnvalue_2
          (for _array_element_2 _outhits_2
            (Utilities|Array|AddUnique (LocalVariables|GetaTempAllCharacters) (.HitActor (Collision|BreakHitResult _array_element_2)))))
        (for _array_element_3 (LocalVariables|GetaTempAllCharacters)
          (Class|BPISTLCharacter|ToggleSelect(Message) _array_element_3 true)
          (Utilities|Array|AddUnique (Variables|Default|GetmSelected%20Actor) _array_element_3))))))

(fn ScreentoLandMapping
  (params (ScreenPosition :type Vector%202D%20Structure%20%28by%20ref%29))
  (bind _returnvalue (Game|GetPlayerController 0))
  (bind (_worldposition _worlddirection) (Class|GameplayStatics|DeprojectScreentoWorld _returnvalue ScreenPosition))
  (bind (_outhit _returnvalue_2) (Collision|LineTraceByChannel _worldposition (+ _worldposition (* _worlddirection 1e+05)) "TraceTypeQuery1" false 0 "ForDuration"))
  (if _returnvalue_2
    (return (.Location (Collision|BreakHitResult _outhit)))
    (else
      (return "0, 0, 0"))))

(event Input|EnhancedActionEvents|EnhancedInputActionIA_SelectActor
  (params (ActionValue :type Boolean) (ElapsedSeconds :type Float%20%28double-precision%29) (TriggeredSeconds :type Float%20%28double-precision%29) (InputAction :type Input%20Action%20Object%20Reference :default "/Game/ConquerTheLand/Input/Actions/IA_SelectActor.IA_SelectActor"))
  (bind (_locationx _locationy) (Game|Player|GetMousePosition))
  (bind (_deltax _deltay) (Class|PlayerController|GetInputMouseDelta))
  (bind _mselected_actor (Variables|Default|GetmSelected%20Actor))
  (:Triggered
    (if (or (!= _deltax 0.0) (!= _deltay 0.0))
      (bind _returnvalue (Class|WidgetLayoutLibrary|GetMousePositiononViewport))
      (Class|BPIHUDBase|DrawSelectBox(Message) (HUD|GetHUD) true (Variables|Default|GetmStartDrawPos) _returnvalue)))
  (:Started
    (bind _returnvalue_2 (Class|WidgetLayoutLibrary|GetMousePositiononViewport))
    (Variables|Default|SetmStartDrawPos _returnvalue_2)
    (Variables|Default|SetmStarSavePos (Math|Vector2D|MakeVector2D _locationx _locationy)))
  (:Completed
    (Class|BPIHUDBase|DrawSelectBox(Message) (HUD|GetHUD) true)
    (if (not (Input|EnhancedActionValues|GetIA_Shift))
      (if (> (Utilities|Array|Length (Variables|Default|GetmSelected%20Actor)) 0)
        (Class|BPISTLCharacter|ToggleSelect(Message) _mselected_actor false)
        (Utilities|Array|Clear _mselected_actor))
      (CallFunction|SelectDrawActor))))