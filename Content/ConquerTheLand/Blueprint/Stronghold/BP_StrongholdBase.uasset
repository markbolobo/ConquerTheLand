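; Base stronghold actor for a conquest game: registers with BP_StrongholdManager, grows its garrison on a timer up to a population cap, and shows the count on camera-facing text.
; Clicking highlights it and notifies the player controller.
; A move order empties the garrison as timed BP_AIBase squads of up to five.
; Arriving units deal damage: friendlies reinforce, enemies subtract soldiers and flip team and icon color at exactly zero.
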(event Custom|CustomEvent
  (if (< (Variables|Default|GetmSoldierNumber) (Utilities|Struct|BreakS_StrongholdInfo (Variables|Default|GetmStrongholdInfo)))
    (Math|Integer|IncrementInt (Variables|Default|GetmSoldierNumber))))

(event EventBeginPlay
  (bind _returnvalue (Actor|GetActorOfClass "/Game/ConquerTheLand/Blueprint/BP_StrongholdManager.BP_StrongholdManager_C"))
  (Variables|Default|SetmStrhManager _returnvalue)
  (Default|AddNewStronghold (Variables|Default|GetmStrhManager) self (Variables|Default|GetmTeamNumber))
  (CallFunction|CheckStrongholdInfo)
  (Utilities|Time|SetTimerbyEvent (delegate Custom|CustomEvent) (Variables|Default|GetmSpawnTime) true))

(event EventTick
  (params (DeltaSeconds :type Float%20%28single-precision%29))
  (Transformation|SetWorldRotation (Variables|Default|GetScene) (Math|Rotator|FindLookatRotation (Transformation|GetWorldLocation (Variables|Default|GetScene)) (Camera|GetCameraLocation (Variables|/Script/Engine.PlayerController|GetPlayerCameraManager (Game|GetPlayerController 0)))) false false)
  (Rendering|Components|TextRender|SetText (Variables|Default|GetTR_SolderNum) (Utilities|Text|ToText(Integer) (Variables|Default|GetmSoldierNumber) false true 2)))

(event MouseInput|EventActorOnClicked
  (params (ButtonPressed :type Key%20Structure :default "None"))
  (CallFunction|RegisterSelectStronghold true)
  (Class|BPICTLController|RegisterSelectActor(Message) (Game|GetPlayerController 0) self))

(event EventRegisterSelectStronghold
  (params (Selected :type Boolean))
  (Development|SetHiddeninGame (Variables|Default|GetSM_SelectedIcon) (not Selected) false))

(event Game|Damage|EventAnyDamage
  (params (Damage :type Float%20%28single-precision%29) (DamageType :type Damage%20Type%20Object%20Reference) (InstigatedBy :type Controller%20Object%20Reference) (DamageCauser :type Actor%20Object%20Reference))
  (bind _returnvalue (Math|Float|Truncate Damage))
  (bind _asbp_aibase (Utilities|Casting|CastToBP_AIBase DamageCauser))
  (if (!= (Variables|/Game/ConquerTheLand/Blueprint/Character/BP_AIBase.BP_AIBase_C|GetmTeam _asbp_aibase) (Variables|Default|GetmTeamNumber))
    (if (>= (Variables|Default|GetmSoldierNumber) _returnvalue)
      (bind _output_get (Variables|Default|SetmSoldierNumber (- (Variables|Default|GetmSoldierNumber) _returnvalue)))
      (else
        (Variables|Default|SetmSoldierNumber (Math|Integer|Absolute(Integer) (- (Variables|Default|GetmSoldierNumber) _returnvalue)))))
    (if (<= _output_get 0)
      (Variables|Default|SetmTeamNumber (Variables|/Game/ConquerTheLand/Blueprint/Character/BP_AIBase.BP_AIBase_C|GetmTeam _asbp_aibase)))
    (Actor|DestroyActor _asbp_aibase :!label _label)
    (CallFunction|CheckStrongholdInfo)
    (elif (and (== (Variables|/Game/ConquerTheLand/Blueprint/Character/BP_AIBase.BP_AIBase_C|GetmTeam _asbp_aibase) (Variables|Default|GetmTeamNumber)) (!= (Variables|/Game/ConquerTheLand/Blueprint/Character/BP_AIBase.BP_AIBase_C|GetmStrongholdNumber _asbp_aibase) (Variables|Default|GetmStrongholdNumber)))
      (Variables|Default|SetmSoldierNumber (+ (Variables|Default|GetmSoldierNumber) (Math|Float|Truncate (Variables|/Game/ConquerTheLand/Blueprint/Character/BP_AIBase.BP_AIBase_C|GetmHP _asbp_aibase))))
      (goto _label))))

(event Custom|CustomEvent_0
  (if (>= (Variables|Default|GetmSoldierNumber) 5)
    (CallFunction|SpawnSoldier (Variables|Default|GetmTarget%20Location) 5.0 5.0)
    (Variables|Default|SetmSoldierNumber (- (Variables|Default|GetmSoldierNumber) 5))
    (else
      (if (> (Variables|Default|GetmSoldierNumber) 0)
        (CallFunction|SpawnSoldier (Variables|Default|GetmTarget%20Location) (Math|Conversions|ToFloat(Integer) (Variables|Default|GetmSoldierNumber)) (Math|Conversions|ToFloat(Integer) (Variables|Default|GetmSoldierNumber)))
        (Variables|Default|SetmSoldierNumber 0))
      (Utilities|Time|ClearandInvalidateTimerbyHandle (Variables|Default|GetmTimerSpawn)))))

(event EventSetSoldierMovetoTarget
  (params (TargetLocation :type Vector :default "0, 0, 0"))
  (Variables|Default|SetmTarget%20Location TargetLocation)
  (Utilities|Time|ClearandInvalidateTimerbyHandle (Variables|Default|GetmTimerSpawn))
  (bind _returnvalue (Utilities|Time|SetTimerbyEvent (delegate Custom|CustomEvent_0) 0.1 true))
  (Variables|Default|SetmTimerSpawn _returnvalue))

(fn ConstructionScript)

(fn SpawnSoldier
  (params (TargetLocation :type Vector) (HP :type Float%20%28double-precision%29) (Damage :type Float%20%28double-precision%29))
  (bind _returnvalue (Game|SpawnActorfromClass "/Game/ConquerTheLand/Blueprint/Character/BP_AIBase.BP_AIBase_C" (Transformation|GetWorldTransform (Variables|Default|GetArrow)) "Undefined" self (Variables|Default|GetmStrongholdNumber) (Variables|Default|GetmTeamNumber) HP Damage 0))
  (if (Utilities|IsValid _returnvalue)
    (Default|MovetoDestination _returnvalue TargetLocation 1e+02)))

(fn CheckStrongholdInfo
  (Rendering|Material|SetMaterial (Variables|Default|GetSM_SelectedIcon) 0 (Utilities|Select :Index (Variables|Default|GetmTeamNumber) :Option%200 "/Game/ConquerTheLand/Art/Materials/MI_IconColor_Green.MI_IconColor_Green" :Option%201 "/Game/ConquerTheLand/Art/Materials/MI_IconColor_Red.MI_IconColor_Red")))

(fn GetIsEnemy
  (params (PlayerTeam :type Integer))
  (return (!= PlayerTeam (Variables|Default|GetmTeamNumber))))