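; Base GameState for Conquer The Land that runs the round timer and ends the match.
; A looping one-second timer counts down from the max round time and pushes it to each PlayerArray member's HUD through ROC_UpdateTime.
; When time runs out or game over is set, the timer stops, BP_StrongholdManager calculates the winner for a debug print, and the level reloads after a delay.
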(event Custom|TE_GameTime
  (if (CallFunction|GetGameOver)
    (Utilities|Time|ClearandInvalidateTimerbyHandle (stale EventBeginPlay _returnvalue_2))
    (bind _winnerplayernumber (Default|CalculateWinner (Variables|Default|GetmStrongholdM)))
    (Development|PrintString (Utilities|String|Append "Winner is : " (Utilities|String|ToString(Integer) _winnerplayernumber)))
    (Utilities|FlowControl|Delay 1e+01)
    (bind _returnvalue (Game|GetCurrentLevelName true))
    (Game|OpenLevel(byName) (Utilities|String|StringToName _returnvalue))
    (else
      (Variables|Default|SetmCurrentTime (- (Variables|Default|GetmCurrentTime) 1.0))
      (CallFunction|ROCUpdateTime)
      (if (<= (Variables|Default|GetmCurrentTime) 0.0)
        (CallFunction|SetGameOver true)
        (Development|PrintString "Game Over")))))

(event Custom|ROC_UpdateTime
  (for _array_element (Variables|Default|GetPlayerArray)
    (Class|BPIHUDBase|UpdateCurrentTime(Message) (HUD|GetHUD (Game|GetPlayerController _array_element)) (Variables|Default|GetmCurrentTime))))

(event EventBeginPlay
  (bind _returnvalue (Actor|GetActorOfClass "/Game/ConquerTheLand/Blueprint/BP_StrongholdManager.BP_StrongholdManager_C"))
  (Variables|Default|SetmStrongholdM _returnvalue)
  (Variables|Default|SetmCurrentTime (Variables|Default|GetmRoundTimeMax))
  (bind _returnvalue_2 (Utilities|Time|SetTimerbyEvent (delegate Custom|TE_GameTime) 1.0 true))
  (Development|PrintString "Game Start"))

(event EventTick
  (params (DeltaSeconds :type Float%20%28single-precision%29)))

(fn ConstructionScript)

(fn GetGameOver
  (return (Variables|Default|GetmGameOver)))

(fn SetGameOver
  (params (GameOver :type Boolean))
  (Variables|Default|SetmGameOver GameOver))