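; BP_StrongholdManager keeps the registry of strongholds and their owning player numbers, and determines which player holds the most.
; AddNewStronghold stores each stronghold with its owner in a map and assigns it a number derived from the map's size.
; CalculateWinner tallies strongholds per owner in a second map, then returns the player with the highest count and that count.
; All logic runs through these two functions, as the event graph is empty.
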(event EventBeginPlay)

(event Collision|EventActorBeginOverlap
  (params (OtherActor :type Actor%20Object%20Reference)))

(event EventTick
  (params (DeltaSeconds :type Float%20%28single-precision%29)))

(fn ConstructionScript)

(fn AddNewStronghold
  (params (NewStronghold :type BP%20Stronghold%20Base%20Object%20Reference%20%28by%20ref%29) (OwnerNumber :type Integer%20%28by%20ref%29))
  (bind _mallstrongholddata (Variables|Default|GetmAllStrongholdData))
  (Utilities|Map|Add _mallstrongholddata NewStronghold OwnerNumber)
  (Variables|/Game/ConquerTheLand/Blueprint/Stronghold/BP_StrongholdBase.BP_StrongholdBase_C|SetmStrongholdNumber NewStronghold (+ (Utilities|Map|Length _mallstrongholddata) 1)))

(fn CalculateWinner
  (bind _values (Utilities|Map|Values (Variables|Default|GetmAllStrongholdData)))
  (for _array_element _values
    (if (.ReturnValue (Utilities|Map|Find (LocalVariables|GetaTempAllStrongholdNum) _array_element))
      (Utilities|Map|Add (LocalVariables|GetaTempAllStrongholdNum) _array_element (+ (.Value (Utilities|Map|Find (LocalVariables|GetaTempAllStrongholdNum) _array_element)) 1))
      (else
        (Utilities|Map|Add (LocalVariables|GetaTempAllStrongholdNum) _array_element 1))))
  (bind _values_2 (Utilities|Map|Values (LocalVariables|GetaTempAllStrongholdNum)))
  (bind _keys (Utilities|Map|Keys (LocalVariables|GetaTempAllStrongholdNum)))
  (return (Utilities|Array|Get(acopy) _keys (.IndexOfMaxValue (Math|Integer|MaxOfIntArray _values_2))) (.MaxValue (Math|Integer|MaxOfIntArray _values_2))))