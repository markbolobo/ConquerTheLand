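; BP_AIBase is a base AI character that can be hovered, clicked to select and ordered to move.
; A click, after a short delay, shows its Cylinder selection marker and registers the actor with the player controller.
; Cursor-over events bound at BeginPlay send or clear the controller's hover message, passing MEnemy on hover.
; MovetoDestination drives movement through AIMoveTo on the character's AI controller.
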(event Custom|OnEndCursorOver_Event
  (params (TouchedActor :type Actor%20Object%20Reference))
  (Class|BPICTLController|ClearHover(Message) (Game|GetPlayerController 0)))

(event Custom|OnBeginCursorOver_Event
  (params (TouchedActor :type Actor%20Object%20Reference))
  (Class|BPICTLController|OnHover(Message) (Game|GetPlayerController 0) (Variables|Default|GetmEnemy)))

(event MouseInput|EventActorOnClicked
  (params (ButtonPressed :type Key%20Structure :default "None"))
  (Utilities|FlowControl|Delay 0.2)
  (CallFunction|ToggleSelect true)
  (Class|BPICTLController|RegisterSelectActor(Message) (Game|GetPlayerController 0) self))

(event EventBeginPlay
  (EventDispatchers|AssignOnBeginCursorOver (delegate Custom|OnBeginCursorOver_Event))
  (EventDispatchers|AssignOnEndCursorOver (delegate Custom|OnEndCursorOver_Event)))

(event EventMovetoDestination
  (params (TargetLocation :type Vector :default "0, 0, 0"))
  (AI|AIMoveTo (AI|GetAIController self) TargetLocation 0 -1.0 "Default" "Default" true true))

(event EventToggleSelect
  (params (Selected :type Boolean))
  (Development|SetHiddeninGame (Variables|Default|GetCylinder) (not Selected) false))

(fn ConstructionScript)