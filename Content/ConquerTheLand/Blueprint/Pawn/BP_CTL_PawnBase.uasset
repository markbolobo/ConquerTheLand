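; Base camera pawn for ConquerTheLand that provides RTS-style edge scrolling and zoom.
; Each Tick reads the mouse position relative to the viewport and offsets the actor in world X or Y when the cursor nears a screen edge.
; Zoom input is smoothed with a delta-time Lerp into a rate that adjusts the spring arm length within clamped limits.
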(event EventBeginPlay)

(event EventTick
  (params (DeltaSeconds :type Float%20%28single-precision%29))
  (CallFunction|SetZoomCamera)
  (CallFunction|SetCameraMoveRight)
  (CallFunction|SetCameraMoveUp))

(fn ConstructionScript)

(fn SetZoomCamera
  (bind _output_get (Variables|Default|SetmZoomRate (Math|Float|Lerp (Variables|Default|GetmZoomRate) (* (Input|EnhancedActionValues|GetIA_Zoom) -1e+02) (* (Utilities|Time|GetWorldDeltaSeconds) 1e+01))))
  (Variables|/Script/Engine.SpringArmComponent|SetTargetArmLength (Variables|Default|GetSpringArm) (Math|Float|Clamp(Float) (+ (Variables|/Script/Engine.SpringArmComponent|GetTargetArmLength (Variables|Default|GetSpringArm)) _output_get) 5e+02 3e+03)))

(fn SetCameraMoveRight
  (bind _returnvalue (Game|GetPlayerController 0))
  (bind _returnvalue_2 (Viewport|GetViewportSize))
  (bind _returnvalue_3 (Utilities|Time|GetWorldDeltaSeconds))
  (bind _scrollspeed (Variables|Default|GetScrollSpeed))
  (bind _locationx (Game|Player|GetMousePosition _returnvalue))
  (bind _returnvalue_4 (* _scrollspeed _returnvalue_3))
  (bind _returnvalue_5 (/ _locationx (.x _returnvalue_2)))
  (if (> _returnvalue_5 0.98)
    (Transformation|AddActorWorldOffset (Math|Vector|MakeVector 0.0 _returnvalue_4 0.0))
    (elif (< _returnvalue_5 0.02)
      (Transformation|AddActorWorldOffset (Math|Vector|MakeVector 0.0 (* _returnvalue_4 -1.0) 0.0)))))

(fn SetCameraMoveUp
  (bind _returnvalue (Game|GetPlayerController 0))
  (bind _returnvalue_2 (Viewport|GetViewportSize))
  (bind _returnvalue_3 (Utilities|Time|GetWorldDeltaSeconds))
  (bind _scrollspeed (Variables|Default|GetScrollSpeed))
  (bind _locationy (Game|Player|GetMousePosition _returnvalue))
  (bind _returnvalue_4 (* _scrollspeed _returnvalue_3))
  (bind _returnvalue_5 (/ _locationy (.y _returnvalue_2)))
  (if (> _returnvalue_5 0.98)
    (Transformation|AddActorWorldOffset (Math|Vector|MakeVector (* _returnvalue_4 -1.0) 0.0 0.0))
    (elif (< _returnvalue_5 0.02)
      (Transformation|AddActorWorldOffset (Math|Vector|MakeVector _returnvalue_4 0.0 0.0)))))