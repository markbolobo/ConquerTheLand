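; BP_Border is a decal-based border actor that draws a rectangular, rounded-corner or circular outline around an area.
; When auto generation is enabled, the construction script derives clamped size, roundness and thickness values, then lays out four line and four corner decals.
; Dynamic materials supply color, thickness and sharpness; square corners hide the corner decals.
; Scaling the actor acts as a resize handle, stepping border size and height before scale resets to one.
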(fn ConstructionScript
  (if (Variables|Settings|GetAutoGenerationEnabled)
    (CallFunction|AutoChangeSizebyScale) ; The scale of this actor automatically resizes the border
    (CallFunction|SetupBorder)))

(fn SetupBorder
  (bind _currentcornerroundness (Variables|Default|GetCurrentCornerRoundness))
  (bind _currentbordersize (Variables|Default|GetCurrentBorderSIze))
  (bind _decalsize (Variables|Default|GetDecalSize))
  (bind _currentcornerroundness_2 (Variables|Default|GetCurrentCornerRoundness))
  (bind _decalsize_2 (Variables|Default|GetDecalSize))
  (bind _currentcornerroundness_3 (Variables|Default|GetCurrentCornerRoundness))
  (bind _currentbordersize_2 (Variables|Default|GetCurrentBorderSIze))
  (bind _currentbordersize_3 (Variables|Default|GetCurrentBorderSIze))
  (bind _decalsize_3 (Variables|Default|GetDecalSize))
  (bind (_x _y) (Math|Vector2D|BreakVector2D _currentbordersize_2))
  (bind _returnvalue (* _currentcornerroundness _decalsize))
  (bind _returnvalue_2 (* _currentcornerroundness_3 _decalsize_2 2.0))
  (bind _returnvalue_3 (- _currentbordersize _returnvalue))
  (bind _returnvalue_4 (- _currentbordersize_3 _returnvalue_2))
  (bind (_x_2 _y_2) (Math|Vector2D|BreakVector2D _returnvalue_3))
  (bind (_x_3 _y_3) (Math|Vector2D|BreakVector2D _returnvalue_3))
  (bind _returnvalue_5 (/ _returnvalue_4 _decalsize_3))
  (bind _returnvalue_6 (* _x_2 0.5))
  (bind _returnvalue_7 (* _y_2 0.5))
  (bind _returnvalue_8 (* _x_2 -0.5))
  (bind _returnvalue_9 (* _y_2 -0.5))
  (bind _returnvalue_10 (* _x_3 0.5))
  (bind _returnvalue_11 (* _y_3 0.5))
  (bind _returnvalue_12 (* _x_3 -0.5))
  (bind _returnvalue_13 (* _y_3 -0.5))
  (CallFunction|SetMainParametrs)
  (Utilities|FlowControl|Sequence
    (:then_0
      ;[0.485 0.1067 0.05466 0.2 12] Sets up  Materials
      (bind _returnvalue_14 (Rendering|Material|CreateDynamicMaterialInstance "/Game/GridBasedBuilder/Blueprints/Border/M_Border_Decal_Line.M_Border_Decal_Line" "None" "None" :!class /Script/Engine.KismetMaterialLibrary))
      (Variables|Default|SetLineDecalMaterial _returnvalue_14)
      (Rendering|Material|SetVectorParameterValue (Variables|Default|GetLineDecalMaterial) "Color" (Variables|Settings|GetBorderColor) :!class /Script/Engine.MaterialInstanceDynamic)
      (Rendering|Material|SetScalarParameterValue (Variables|Default|GetLineDecalMaterial) "CornerRoundness" (Variables|Default|GetLineThicknessFactor) :!class /Script/Engine.MaterialInstanceDynamic)
      (Rendering|Material|SetScalarParameterValue (Variables|Default|GetLineDecalMaterial) "Density" (Variables|Settings|GetBorderSharpness) :!class /Script/Engine.MaterialInstanceDynamic)
      (Rendering|Components|Decal|SetDecalMaterial (Variables|Components|GetLine_T) (Variables|Default|GetLineDecalMaterial))
      (if (or (Variables|Settings|GetRoundArea) (Variables|Settings|GetRoundedCorners))
        (bind _returnvalue_15 (Rendering|Material|CreateDynamicMaterialInstance "/Game/GridBasedBuilder/Blueprints/Border/M_Border_Decal_Corner.M_Border_Decal_Corner" "None" "None" :!class /Script/Engine.KismetMaterialLibrary))
        (Variables|Default|SetCornerDecalMaterial _returnvalue_15)
        (Rendering|Material|SetVectorParameterValue (Variables|Default|GetCornerDecalMaterial) "Color" (Variables|Settings|GetBorderColor) :!class /Script/Engine.MaterialInstanceDynamic)
        (Rendering|Material|SetScalarParameterValue (Variables|Default|GetCornerDecalMaterial) "CornerRoundness" (Variables|Default|GetLineThicknessFactor) :!class /Script/Engine.MaterialInstanceDynamic)
        (Rendering|Material|SetScalarParameterValue (Variables|Default|GetCornerDecalMaterial) "Density" (Variables|Settings|GetBorderSharpness) :!class /Script/Engine.MaterialInstanceDynamic)
        (Rendering|Components|Decal|SetDecalMaterial (Variables|Components|GetCorner_TR) (Variables|Default|GetCornerDecalMaterial))
        (else
          (Rendering|SetVisibility (Variables|Components|GetCorner_TL) false false))))
    (:then_1
      ;[0.485 0.1067 0.05466 0.2 12] Sets up  Rectangle Area with Round Corners or Round Area
      (if (or (Variables|Settings|GetRoundArea) (Variables|Settings|GetRoundedCorners))
        (Transformation|SetRelativeScale3D (Variables|Components|GetCorner_TR) (Math|Vector|MakeVector (Variables|Default|GetCurrentBorderHeight) _currentcornerroundness_2 _currentcornerroundness_2))
        (Transformation|SetRelativeScale3D (Variables|Components|GetLine_B) (Math|Vector|MakeVector (Variables|Default|GetCurrentBorderHeight) (Math|Float|Clamp(Float) (.y _returnvalue_5) 0.0 (.y _returnvalue_5)) (Variables|Default|GetCurrentCornerRoundness)))
        (Transformation|SetRelativeScale3D (Variables|Components|GetLine_L) (Math|Vector|MakeVector (Variables|Default|GetCurrentBorderHeight) (Math|Float|Clamp(Float) (.x _returnvalue_5) 0.0 (.x _returnvalue_5)) (Variables|Default|GetCurrentCornerRoundness)))
        (Transformation|SetRelativeLocation (Variables|Components|GetLine_T) (Math|Vector|MakeVector _returnvalue_6 0.0 0.0) false false)
        (Transformation|SetRelativeLocation (Variables|Components|GetLine_B) (Math|Vector|MakeVector _returnvalue_8 0.0 0.0) false false)
        (Transformation|SetRelativeLocation (Variables|Components|GetLine_R) (Math|Vector|MakeVector 0.0 _returnvalue_7 0.0) false false)
        (Transformation|SetRelativeLocation (Variables|Components|GetLine_L) (Math|Vector|MakeVector 0.0 _returnvalue_9 0.0) false false)
        (Transformation|SetRelativeLocation (Variables|Components|GetCorner_TR) (Math|Vector|MakeVector _returnvalue_10 _returnvalue_11 0.0) false false)
        (Transformation|SetRelativeLocation (Variables|Components|GetCorner_TL) (Math|Vector|MakeVector _returnvalue_12 _returnvalue_11 0.0) false false)
        (Transformation|SetRelativeLocation (Variables|Components|GetCorner_BR) (Math|Vector|MakeVector _returnvalue_12 _returnvalue_13 0.0) false false)
        (Transformation|SetRelativeLocation (Variables|Components|GetCorner_BL) (Math|Vector|MakeVector _returnvalue_10 _returnvalue_13 0.0) false false)
        (else
          ;[0.485 0.1067 0.05466 0.2 12] Sets up  Rectangle Area with Rectangle Corners
          (Transformation|SetRelativeScale3D (Variables|Components|GetLine_B) (Math|Vector|MakeVector (Variables|Default|GetCurrentBorderHeight) (/ _y (Variables|Default|GetDecalSize)) (Variables|Default|GetCurrentCornerRoundness)))
          (Transformation|SetRelativeScale3D (Variables|Components|GetLine_L) (Math|Vector|MakeVector (Variables|Default|GetCurrentBorderHeight) (/ (- _x (* (Variables|Default|GetDecalSize) (Variables|Default|GetLineThicknessFactor) (Variables|Default|GetCurrentCornerRoundness) 2.0)) (Variables|Default|GetDecalSize)) (Variables|Default|GetCurrentCornerRoundness)))
          (Transformation|SetRelativeLocation (Variables|Components|GetLine_T) (Math|Vector|MakeVector _returnvalue_6 0.0 0.0) false false)
          (Transformation|SetRelativeLocation (Variables|Components|GetLine_B) (Math|Vector|MakeVector _returnvalue_8 0.0 0.0) false false)
          (Transformation|SetRelativeLocation (Variables|Components|GetLine_R) (Math|Vector|MakeVector 0.0 _returnvalue_7 0.0) false false)
          (Transformation|SetRelativeLocation (Variables|Components|GetLine_L) (Math|Vector|MakeVector 0.0 _returnvalue_9 0.0) false false))))))

(fn AutoChangeSizebyScale
  (bind _returnvalue (Class|Actor|GetActorRelativeScale3D))
  (bind (_x _y _z) (Math|Vector|BreakVector _returnvalue))
  (bind (_x_2 _y_2 _z_2) (Math|Vector|BreakVector _returnvalue))
  (if (Math|Vector|Equal(Vector) (Class|Actor|GetActorRelativeScale3D) "1.000000,1.000000,1.000000" 0.01)
    _
    (else
      (Variables|Settings|SetBorderSIze (Math|Vector2D|MakeVector2D (Math|Float|SelectFloat (Math|Float|SelectFloat (.X (Math|Vector2D|BreakVector2D (Variables|Settings|GetBorderSIze))) (+ (.X (Math|Vector2D|BreakVector2D (Variables|Settings|GetBorderSIze))) (* (Math|Float|SelectFloat -1.0 1.0 (< _x 1.0)) (Math|Float|Clamp(Float) (/ (.X (Math|Vector2D|BreakVector2D (Variables|Settings|GetBorderSIze))) 2e+01) 1e+01 1e+04))) (== _x_2 1.0)) 0.0 (>= (Math|Float|SelectFloat (.X (Math|Vector2D|BreakVector2D (Variables|Settings|GetBorderSIze))) (+ (.X (Math|Vector2D|BreakVector2D (Variables|Settings|GetBorderSIze))) (* (Math|Float|SelectFloat -1.0 1.0 (< _x 1.0)) (Math|Float|Clamp(Float) (/ (.X (Math|Vector2D|BreakVector2D (Variables|Settings|GetBorderSIze))) 2e+01) 1e+01 1e+04))) (== _x_2 1.0)) 0.0)) (Math|Float|SelectFloat (Math|Float|SelectFloat (.Y (Math|Vector2D|BreakVector2D (Variables|Settings|GetBorderSIze))) (+ (.Y (Math|Vector2D|BreakVector2D (Variables|Settings|GetBorderSIze))) (* (Math|Float|SelectFloat -1.0 1.0 (< _y 1.0)) (Math|Float|Clamp(Float) (/ (.Y (Math|Vector2D|BreakVector2D (Variables|Settings|GetBorderSIze))) 2e+01) 1e+01 1e+04))) (== _y_2 1.0)) 0.0 (>= (Math|Float|SelectFloat (.Y (Math|Vector2D|BreakVector2D (Variables|Settings|GetBorderSIze))) (+ (.Y (Math|Vector2D|BreakVector2D (Variables|Settings|GetBorderSIze))) (* (Math|Float|SelectFloat -1.0 1.0 (< _y 1.0)) (Math|Float|Clamp(Float) (/ (.Y (Math|Vector2D|BreakVector2D (Variables|Settings|GetBorderSIze))) 2e+01) 1e+01 1e+04))) (== _y_2 1.0)) 0.0))))
      (Variables|Settings|SetBorderHeight (Math|Float|SelectFloat (Math|Float|SelectFloat (Variables|Settings|GetBorderHeight) (+ (Variables|Settings|GetBorderHeight) (* (Math|Float|SelectFloat -1.0 1.0 (< _z 1.0)) (Math|Float|Clamp(Float) (/ (Variables|Settings|GetBorderHeight) 2e+01) 0.1 5e+01))) (== _z_2 1.0)) 0.0 (>= (Math|Float|SelectFloat (Variables|Settings|GetBorderHeight) (+ (Variables|Settings|GetBorderHeight) (* (Math|Float|SelectFloat -1.0 1.0 (< _z 1.0)) (Math|Float|Clamp(Float) (/ (Variables|Settings|GetBorderHeight) 2e+01) 0.1 5e+01))) (== _z_2 1.0)) 0.0)))))
  (Transformation|SetActorScale3D "1.000000,1.000000,1.000000") ; Reset actor Scale
)

(fn SetMainParametrs
  (bind _decalsize (Variables|Default|GetDecalSize))
  (bind _bordersize (Variables|Settings|GetBorderSIze))
  (bind _x (Math|Vector2D|BreakVector2D _bordersize))
  (bind _returnvalue (* _decalsize 2.0))
  (Utilities|FlowControl|Sequence
    (:then_0
      (Variables|Default|SetCurrentBorderSIze (Class|KismetMathLibrary|GetAbs2D (Variables|Settings|GetBorderSIze)))
      (if (Variables|Settings|GetRoundArea)
        (Variables|Default|SetCurrentBorderSIze (Math|Vector2D|MakeVector2D _x _x))))
    (:then_1
      (Variables|Settings|SetLineThickness (Math|Float|Clamp(Float) (Variables|Settings|GetLineThickness) 0.01 (Variables|Settings|GetLineThickness)))
      (Variables|Default|SetCurrentBorderHeight (/ (Math|Float|Absolute(Float) (Variables|Settings|GetBorderHeight)) 2e+02))
      (Variables|Default|SetCurrentCornerRoundness (Math|Float|Clamp(Float) (Math|Float|SelectFloat (/ (.X (Math|Vector2D|BreakVector2D (Variables|Default|GetCurrentBorderSIze))) _returnvalue) (Math|Float|Clamp(Float) (/ (Variables|Settings|GetCornerRoundness) (Variables|Default|GetDecalSize)) 0.0 (Math|Float|SelectFloat (/ (.Y (Math|Vector2D|BreakVector2D (Variables|Default|GetCurrentBorderSIze))) _returnvalue) (/ (.X (Math|Vector2D|BreakVector2D (Variables|Default|GetCurrentBorderSIze))) _returnvalue) (>= (.X (Math|Vector2D|BreakVector2D (Variables|Default|GetCurrentBorderSIze))) (.Y (Math|Vector2D|BreakVector2D (Variables|Default|GetCurrentBorderSIze)))))) (Variables|Settings|GetRoundArea)) 0.01 (Math|Float|SelectFloat (/ (.X (Math|Vector2D|BreakVector2D (Variables|Default|GetCurrentBorderSIze))) _returnvalue) (Math|Float|Clamp(Float) (/ (Variables|Settings|GetCornerRoundness) (Variables|Default|GetDecalSize)) 0.0 (Math|Float|SelectFloat (/ (.Y (Math|Vector2D|BreakVector2D (Variables|Default|GetCurrentBorderSIze))) _returnvalue) (/ (.X (Math|Vector2D|BreakVector2D (Variables|Default|GetCurrentBorderSIze))) _returnvalue) (>= (.X (Math|Vector2D|BreakVector2D (Variables|Default|GetCurrentBorderSIze))) (.Y (Math|Vector2D|BreakVector2D (Variables|Default|GetCurrentBorderSIze)))))) (Variables|Settings|GetRoundArea))))
      (Variables|Default|SetLineThicknessFactor (Math|Float|Clamp(Float) (/ (/ 1.0 (Math|Float|Clamp(Float) (Variables|Default|GetCurrentCornerRoundness) 0.01 (Variables|Default|GetCurrentCornerRoundness))) (Variables|Settings|GetLineThickness)))))))