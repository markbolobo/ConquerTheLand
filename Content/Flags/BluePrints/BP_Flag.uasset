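; Customizable flag actor with a skeletal-mesh cloth, swappable base and pole endings, built in the construction script.
; Enum-keyed data tables supply meshes and textures, which helper functions apply to a dynamic material instance for style, pattern, decoration, emblem, folds, damage and dirt.
; With UseRandomGenerator on, Randomize derives the look from a seeded stream instead, skipping damage and visibility setup.
; NextFlag and PreviousFlag step the seed and re-randomize.
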(fn ConstructionScript
  (bind _flagscale (Variables|Main|GetFlagScale))
  (bind _sm_base (Variables|Default|GetSM_Base))
  (bind _e_flag_material_to_instance (Variables|Main|GetE_Flag_Material_To_Instance))
  ;[1 1 1] Setup Mesh
  (Math|Random|SetRandomStreamSeed (Variables|RandomGenerator|GetStream) (Variables|RandomGenerator|GetNew%20Seed))
  (if (not (Variables|RandomGenerator|GetuseRandomGenerator?))
    (Transformation|SetWorldScale3D (Variables|Default|GetFlag_Pivot) (Math|Vector|MakeVector _flagscale _flagscale _flagscale))
    (switch Utilities|FlowControl|Switch|SwitchonE_FlagHoldersVisibility (Variables|Main|GetFlagVisibility)
      (:NewEnumerator0
        _)
      (:NewEnumerator1
        (Rendering|SetVisibility (Variables|Default|GetEnds) false true))
      (:NewEnumerator2
        (Rendering|SetVisibility (Variables|Default|GetSM_Mid) false true))
      (:NewEnumerator3
        (Rendering|SetVisibility (Variables|Default|GetSM_Mid) false true)))
    (if (Variables|Main|Getuse%20Base?)
      (Rendering|SetVisibility _sm_base true false)
      (else
        (Rendering|SetVisibility _sm_base false false)))
    (CallFunction|SetBaseMesh _sm_base)
    (CallFunction|SetEndings (Variables|Default|GetSM_Top) (Variables|Default|GetSM_Side_A) (Variables|Default|GetSM_Side_B))
    ;[1 1 1] Basic Material or with Dirt and Gradient?
    (bind _returnvalue (Utilities|GetDataTableRow (Variables|DataTables|GetDT_Flag_Material_To_Instance) (Utilities|String|StringToName (Utilities|String|EnumtoString _e_flag_material_to_instance)))
      (:then
        (Variables|Default|SetshowDirtandGradient (Utilities|Enum|Equal(Enum) _e_flag_material_to_instance "NewEnumerator1"))
        ;[1 1 1] Material Setup
        (bind _returnvalue_2 (Rendering|Material|CreateDynamicMaterialInstance (Variables|Default|GetSK_Flag) 0 (.MaterialToInstance (Utilities|Struct|BreakS_Flag_Material_To_Instance _returnvalue)) "None" :!class /Script/Engine.PrimitiveComponent))
        (Variables|Default|SetREF_Dynamic_Material _returnvalue_2)
        (CallFunction|SetStyle)
        (CallFunction|SetPattern)
        (CallFunction|SetDecorations)
        (CallFunction|SetEmblems)
        (CallFunction|SetNormal)
        (CallFunction|SetDamage)
        (Rendering|Material|SetVectorParameterValueonMaterials (Variables|Default|GetSK_Flag) "Flag Color" (Math|Conversions|ToVector(LinearColor) (Variables|Main|GetFlag%20Color)))
        (Rendering|Material|SetVectorParameterValueonMaterials (Variables|Default|GetSK_Flag) "Flag Border Tint" (Math|Conversions|ToVector(LinearColor) (Variables|0-Pattern|GetFlag%20Border%20Tint)))
        (Rendering|Material|SetScalarParameterValueonMaterials (Variables|Default|GetSK_Flag) "Roughness from Color" (Variables|Main|GetRoughnessFromColor))
        ;[1 1 1] Dirt and Gradient if appropreate material is choosen
        (if (Variables|Default|GetshowDirtandGradient)
          (CallFunction|SetDirtMasks)
          (Rendering|Material|SetVectorParameterValueonMaterials (Variables|Default|GetSK_Flag) "Gradient Bot" (Math|Conversions|ToVector(LinearColor) (Variables|5-Dirt&Gradient|GetGradient%20Bot)))
          (Rendering|Material|SetVectorParameterValueonMaterials (Variables|Default|GetSK_Flag) "Gradient Top" (Math|Conversions|ToVector(LinearColor) (Variables|5-Dirt&Gradient|GetGradient%20Top))))))
    (else
      (RandomGenerator|Randomize))))

(fn SetEmblems
  (bind _returnvalue (Utilities|GetDataTableRow (Variables|DataTables|GetDT_Flag_Emblems) (Utilities|String|StringToName (Utilities|String|EnumtoString (Variables|2-Emblem|GetE_Flag_Emblems))))
    (:then
      (Rendering|Material|SetScalarParameterValueonMaterials (Variables|Default|GetSK_Flag) "Scale X" (Variables|2-Emblem|GetScale%20Emblem%20X))
      (Rendering|Material|SetScalarParameterValueonMaterials (Variables|Default|GetSK_Flag) "Scale Y" (Variables|2-Emblem|GetScale%20Emblem%20Y))
      (Rendering|Material|SetScalarParameterValueonMaterials (Variables|Default|GetSK_Flag) "Shift X" (Variables|2-Emblem|GetShift%20Emblem%20X))
      (Rendering|Material|SetScalarParameterValueonMaterials (Variables|Default|GetSK_Flag) "Emblem Opacity" (Variables|2-Emblem|GetEmblem%20Opacity))
      (Rendering|Material|SetScalarParameterValueonMaterials (Variables|Default|GetSK_Flag) "Shift Y" (Variables|2-Emblem|GetShift%20Emblem%20Y))
      (Rendering|Material|SetTextureParameterValue (Variables|Default|GetREF_Dynamic_Material) "Emblem" (.FlagEmblemTexture (Utilities|Struct|BreakS_Flag_Emblems _returnvalue)))
      (Rendering|Material|SetVectorParameterValue (Variables|Default|GetREF_Dynamic_Material) "Emblem Color" (Variables|2-Emblem|GetEmblem%20Color) :!class /Script/Engine.MaterialInstanceDynamic)
      (return))))

(fn SetDecorations
  (bind _returnvalue (Utilities|GetDataTableRow (Variables|DataTables|GetDT_Flag_Decorations) (Utilities|String|StringToName (Utilities|String|EnumtoString (Variables|1-Decoratives|GetE_Flag_Decorations))))
    (:then
      (Rendering|Material|SetScalarParameterValueonMaterials (Variables|Default|GetSK_Flag) "Deco Pattern Opacity" (Variables|1-Decoratives|GetDeco%20Opacity))
      (Rendering|Material|SetScalarParameterValueonMaterials (Variables|Default|GetSK_Flag) "Scale X Deco Pattern" (Variables|1-Decoratives|GetScale%20X))
      (Rendering|Material|SetScalarParameterValueonMaterials (Variables|Default|GetSK_Flag) "Scale Y Deco Pattern" (Variables|1-Decoratives|GetScale%20Y))
      (Rendering|Material|SetScalarParameterValueonMaterials (Variables|Default|GetSK_Flag) "Shift X Deco Pattern" (Variables|1-Decoratives|GetShift%20X))
      (Rendering|Material|SetScalarParameterValueonMaterials (Variables|Default|GetSK_Flag) "Shift Y Deco Pattern" (Variables|1-Decoratives|GetShift%20Y))
      (Rendering|Material|SetVectorParameterValueonMaterials (Variables|Default|GetSK_Flag) "Deco Pattern Color" (Math|Conversions|ToVector(LinearColor) (Variables|1-Decoratives|GetDeco%20Color)))
      (Rendering|Material|SetTextureParameterValue (Variables|Default|GetREF_Dynamic_Material) "Deco Pattern" (.FlagDecorationTexture (Utilities|Struct|BreakS_Flag_Decorations _returnvalue)))
      (return))))

(fn SetPattern
  (switch Utilities|FlowControl|Switch|SwitchonE_SwitchOpacityPattern (Variables|0-Pattern|GetE_Flag_Opacity_Switcher)
    (:NewEnumerator0
      (Variables|0-Pattern|SetMain%20Pattern%20Opacity 0.0)
      (Variables|0-Pattern|SetPatternOnBorder 0.0))
    (:NewEnumerator1
      (Variables|0-Pattern|SetMain%20Pattern%20Opacity 1.0)
      (Variables|0-Pattern|SetPatternOnBorder 1.0))
    (:NewEnumerator2
      _))
  (Rendering|Material|SetScalarParameterValueonMaterials (Variables|Default|GetSK_Flag) "PatternOnBorder" (Variables|0-Pattern|GetPatternOnBorder))
  (Rendering|Material|SetScalarParameterValueonMaterials (Variables|Default|GetSK_Flag) "Pattern Tile" (Variables|0-Pattern|GetPattern%20Tile))
  (Rendering|Material|SetScalarParameterValueonMaterials (Variables|Default|GetSK_Flag) "Main Pattern Opacity" (Variables|0-Pattern|GetMain%20Pattern%20Opacity))
  (Rendering|Material|SetScalarParameterValueonMaterials (Variables|Default|GetSK_Flag) "Pattern Rotation" (Variables|0-Pattern|GetPattern%20Rotation))
  (bind _returnvalue (Utilities|GetDataTableRow (Variables|DataTables|GetDT_Flag_Patterns) (Utilities|String|StringToName (Utilities|String|EnumtoString (Variables|0-Pattern|GetE_Flag_Patterns))))
    (:then
      (Rendering|Material|SetTextureParameterValue (Variables|Default|GetREF_Dynamic_Material) "Flag Texture" (.FlagPattern (Utilities|Struct|BreakS_Flag_Patterns _returnvalue)))
      (return))))

(fn SetStyle
  (bind _returnvalue (Utilities|GetDataTableRow (Variables|DataTables|GetDT_Flag_Style) (Utilities|String|StringToName (Utilities|String|EnumtoString (Variables|Main|GetE_Flag_Style))))
    (:then
      (Rendering|Material|SetTextureParameterValue (Variables|Default|GetREF_Dynamic_Material) "Alpha" (.FlagStyleAlpha (Utilities|Struct|BreakS_Flag_Style _returnvalue)))
      (Rendering|Material|SetTextureParameterValue (Variables|Default|GetREF_Dynamic_Material) "Flag_Border_Mask" (.FlagStyleBorder (Utilities|Struct|BreakS_Flag_Style _returnvalue)))
      (return))))

(fn SetNormal
  (bind _returnvalue (Utilities|GetDataTableRow (Variables|DataTables|GetDT_Flag_Normals) (Utilities|String|StringToName (Utilities|String|EnumtoString (Variables|3-Folds|GetE_Flag_Normals%28Folds%29))))
    (:then
      (Rendering|Material|SetTextureParameterValue (Variables|Default|GetREF_Dynamic_Material) "Normal" (.FlagNormalTexture (Utilities|Struct|BreakS_Flag_Normals _returnvalue)))
      (Rendering|Material|SetScalarParameterValueonMaterials (Variables|Default|GetSK_Flag) "Normal Strenght" (Variables|3-Folds|GetNormal%20Strenght))
      (return))))

(fn SetDamage
  (bind _returnvalue (Utilities|GetDataTableRow (Variables|DataTables|GetDT_Flag_Damage) (Utilities|String|StringToName (Utilities|String|EnumtoString (Variables|4-Damage|GetE_Flag_Damage))))
    (:then
      (Rendering|Material|SetTextureParameterValue (Variables|Default|GetREF_Dynamic_Material) "Damage Masks" (.FlagDamageTexture (Utilities|Struct|BreakS_Flag_Damage _returnvalue)))
      (Rendering|Material|SetScalarParameterValueonMaterials (Variables|Default|GetSK_Flag) "Destroyed Mask Power" (Variables|4-Damage|GetDestroyed%20Mask%20Power))
      (Rendering|Material|SetScalarParameterValueonMaterials (Variables|Default|GetSK_Flag) "Shift X Damage" (Variables|4-Damage|GetShift%20X%20Damage))
      (Rendering|Material|SetScalarParameterValueonMaterials (Variables|Default|GetSK_Flag) "Shift Y Damage" (Variables|4-Damage|GetShift%20Y%20Damage))
      (return))))

(fn SetBaseMesh
  (params (Base :type Static%20Mesh%20Component%20Object%20Reference))
  (bind _returnvalue (Utilities|GetDataTableRow (Variables|DataTables|GetDT_Flag_Base) (Utilities|String|StringToName (Utilities|String|EnumtoString (Variables|Main|GetE_Flag_Base))))
    (:then
      (Components|StaticMesh|SetStaticMesh Base (.Static_Mesh (Utilities|Struct|BreakS_Flag_Base _returnvalue)))
      (return))))

(fn SetEndings
  (params (Top :type Static%20Mesh%20Component%20Object%20Reference) (Side%20A :type Static%20Mesh%20Component%20Object%20Reference) (Side%20B :type Static%20Mesh%20Component%20Object%20Reference))
  (bind _returnvalue (Utilities|GetDataTableRow (Variables|DataTables|GetDT_Flag_Endings) (Utilities|String|StringToName (Utilities|String|EnumtoString (Variables|Main|GetE_Flag_Endings))))
    (:then
      (for _array_element (Utilities|Array|MakeArray Top Side%20A Side%20B)
        (Components|StaticMesh|SetStaticMesh _array_element (.Static_Mesh (Utilities|Struct|BreakS_Flag_Endings _returnvalue))))
      (return))))

(fn SetDirtMasks
  (bind _returnvalue (Utilities|GetDataTableRow (Variables|DataTables|GetDT_Dirt_Masks) (Utilities|String|StringToName (Utilities|String|EnumtoString (Variables|5-Dirt&Gradient|GetE_Dirt_Masks))))
    (:then
      (Rendering|Material|SetTextureParameterValue (Variables|Default|GetREF_Dynamic_Material) "Dirt Mask" (.DirtMaskTexture (Utilities|Struct|BreakS_Dirt_Mask _returnvalue)))
      (Rendering|Material|SetScalarParameterValueonMaterials (Variables|Default|GetSK_Flag) "Dirt Power" (Variables|5-Dirt&Gradient|GetDirt%20Power)))))

(fn Randomize
  (bind _stream (Variables|RandomGenerator|GetStream))
  (bind _stream_2 (Variables|RandomGenerator|GetStream))
  (bind _stream_3 (Variables|RandomGenerator|GetStream))
  (bind _stream_4 (Variables|RandomGenerator|GetStream))
  (bind _stream_5 (Variables|RandomGenerator|GetStream))
  (bind _stream_6 (Variables|RandomGenerator|GetStream))
  (bind _stream_7 (Variables|RandomGenerator|GetStream))
  (bind _returnvalue (Math|Random|RandomUnitVectorfromStream _stream_6))
  (bind _returnvalue_2 (Math|Random|RandomUnitVectorfromStream _stream_7))
  (bind _returnvalue_3 (Math|Random|RandomFloatinRangefromStream 0.0 1.0 _stream))
  (bind _returnvalue_4 (Math|Random|RandomUnitVectorfromStream _stream_3))
  (bind _returnvalue_5 (Math|Random|RandomUnitVectorfromStream _stream_2))
  (bind _returnvalue_6 (Math|Random|RandomUnitVectorfromStream _stream_4))
  (bind _returnvalue_7 (Math|Random|RandomUnitVectorfromStream _stream_5))
  (if (Variables|RandomGenerator|GetuseRandomGenerator?)
    (Utilities|FlowControl|Sequence
      (:then_0
        ;[1 1 1] Setup Stream Seed, Mesh Style
        (bind _output_get (Variables|Main|SetFlagScale (Math|Random|RandomFloatinRangefromStream 0.8 1.0 (Variables|RandomGenerator|GetStream))))
        (Transformation|SetWorldScale3D (Variables|Default|GetFlag_Pivot) (Math|Vector|MakeVector _output_get _output_get _output_get))
        (bind _returnvalue_8 (CallFunction|RandomEnum (|GetNumEnumEntries) (Variables|RandomGenerator|GetStream)))
        (Variables|Main|SetE_Flag_Base (Utilities|Enum|ByteToEnumE_Flag_Base _returnvalue_8))
        (CallFunction|SetBaseMesh (Variables|Default|GetSM_Base))
        (bind _returnvalue_9 (CallFunction|RandomEnum (|GetNumEnumEntries) (Variables|RandomGenerator|GetStream)))
        (Variables|Main|SetE_Flag_Endings (Utilities|Enum|ByteToEnumE_Flag_Endings _returnvalue_9))
        (CallFunction|SetEndings (Variables|Default|GetSM_Top) (Variables|Default|GetSM_Side_A) (Variables|Default|GetSM_Side_B))
        (bind _returnvalue_10 (CallFunction|RandomEnum (|GetNumEnumEntries) (Variables|RandomGenerator|GetStream)))
        (bind _output_get_2 (Variables|Main|SetE_Flag_Material_To_Instance (Utilities|Enum|ByteToEnumE_Flag_Material_To_Instance _returnvalue_10)))
        (bind _returnvalue_11 (Utilities|GetDataTableRow (Variables|DataTables|GetDT_Flag_Material_To_Instance) (Utilities|String|StringToName (Utilities|String|EnumtoString _output_get_2)))
          (:then
            (bind _returnvalue_12 (Rendering|Material|CreateDynamicMaterialInstance (Variables|Default|GetSK_Flag) 0 (.MaterialToInstance (Utilities|Struct|BreakS_Flag_Material_To_Instance _returnvalue_11)) "None" :!class /Script/Engine.PrimitiveComponent))
            (Variables|Default|SetshowDirtandGradient (Utilities|Enum|Equal(Enum) _output_get_2 "NewEnumerator1"))
            (Variables|Default|SetREF_Dynamic_Material _returnvalue_12)
            (bind _returnvalue_13 (CallFunction|RandomEnum (|GetNumEnumEntries) (Variables|RandomGenerator|GetStream)))
            (Variables|Main|SetE_Flag_Style (Utilities|Enum|ByteToEnumE_Flag_Style _returnvalue_13))
            (CallFunction|SetStyle))))
      (:then_1
        ;[1 1 1] Random Pattern
        (bind _returnvalue_14 (CallFunction|RandomEnum (|GetNumEnumEntries) (Variables|RandomGenerator|GetStream)))
        (Variables|0-Pattern|SetE_Flag_Patterns (Utilities|Enum|ByteToEnumE_Flag_Patterns _returnvalue_14))
        (bind _returnvalue_15 (CallFunction|RandomEnum (|GetNumEnumEntries) (Variables|RandomGenerator|GetStream)))
        (Variables|0-Pattern|SetE_Flag_Opacity_Switcher (Utilities|Enum|ByteToEnumE_SwitchOpacityPattern _returnvalue_15))
        (Variables|0-Pattern|SetMain%20Pattern%20Opacity _returnvalue_3)
        (Variables|0-Pattern|SetPatternOnBorder _returnvalue_3)
        (Variables|0-Pattern|SetPattern%20Tile (Math|Random|RandomFloatinRangefromStream 1.0 8.0 (Variables|RandomGenerator|GetStream)))
        (Variables|0-Pattern|SetPattern%20Rotation (Math|Random|RandomFloatinRangefromStream 0.0 3.6e+02 (Variables|RandomGenerator|GetStream)))
        (Variables|0-Pattern|SetFlag%20Border%20Tint (Utilities|Struct|MakeLinearColor (.x _returnvalue_4) (.y _returnvalue_4) (.z _returnvalue_4) (Math|Random|RandomFloatinRangefromStream 0.0 1.0 _stream_3)))
        (CallFunction|SetPattern))
      (:then_2
        ;[1 1 1] Random Decorative Pattern
        (bind _returnvalue_16 (CallFunction|RandomEnum (|GetNumEnumEntries) (Variables|RandomGenerator|GetStream)))
        (Variables|1-Decoratives|SetE_Flag_Decorations (Utilities|Enum|ByteToEnumE_Flag_Decorations _returnvalue_16))
        (Variables|1-Decoratives|SetDeco%20Color (Utilities|Struct|MakeLinearColor (.x _returnvalue_5) (.y _returnvalue_5) (.z _returnvalue_5) (Math|Random|RandomFloatinRangefromStream 0.0 1.0 _stream_2)))
        (Variables|1-Decoratives|SetDeco%20Opacity (Math|Random|RandomFloatinRangefromStream 0.0 1.0 (Variables|RandomGenerator|GetStream)))
        (bind _output_get_3 (Variables|Default|SetRandom%20Scale%20Decorations (Math|Random|RandomFloatinRangefromStream 0.9 1.1 (Variables|RandomGenerator|GetStream))))
        (Variables|1-Decoratives|SetScale%20X _output_get_3)
        (Variables|1-Decoratives|SetScale%20Y _output_get_3)
        (Variables|1-Decoratives|SetShift%20X 0.0)
        (Variables|1-Decoratives|SetShift%20Y 0.0)
        (CallFunction|SetDecorations))
      (:then_3
        ;[1 1 1] Random Emblem
        (bind _returnvalue_17 (CallFunction|RandomEnum (|GetNumEnumEntries) (Variables|RandomGenerator|GetStream)))
        (Variables|2-Emblem|SetE_Flag_Emblems (Utilities|Enum|ByteToEnumE_Flag_Emblems _returnvalue_17))
        (Variables|2-Emblem|SetEmblem%20Color (Utilities|Struct|MakeLinearColor (.x _returnvalue_6) (.y _returnvalue_6) (.z _returnvalue_6) (Math|Random|RandomFloatinRangefromStream 0.0 1.0 _stream_4)))
        (Variables|2-Emblem|SetEmblem%20Opacity (Math|Random|RandomFloatinRangefromStream 0.8 1.0 (Variables|RandomGenerator|GetStream)))
        (bind _output_get_4 (Variables|Default|SetRandom%20Scale%20Emblem (Math|Random|RandomFloatinRangefromStream 0.4 0.6 (Variables|RandomGenerator|GetStream))))
        (Variables|2-Emblem|SetScale%20Emblem%20X _output_get_4)
        (Variables|2-Emblem|SetScale%20Emblem%20Y _output_get_4)
        (CallFunction|SetEmblems))
      (:then_4
        ;[1 1 1] Random Folds
        (bind _returnvalue_18 (CallFunction|RandomEnum (|GetNumEnumEntries) (Variables|RandomGenerator|GetStream)))
        (Variables|3-Folds|SetE_Flag_Normals%28Folds%29 (Utilities|Enum|ByteToEnumE_Flag_Normals _returnvalue_18))
        (Variables|3-Folds|SetNormal%20Strenght (Math|Random|RandomFloatinRangefromStream 0.0 1.0 (Variables|RandomGenerator|GetStream)))
        ;[1 1 1] Color and rest
        (Variables|Main|SetFlag%20Color (Utilities|Struct|MakeLinearColor (.x _returnvalue) (.y _returnvalue) (.z _returnvalue) (Math|Random|RandomFloatinRangefromStream 0.0 1.0 _stream_6)))
        (Variables|Main|SetRoughnessFromColor (Math|Random|RandomFloatinRangefromStream 0.7 1.6 (Variables|RandomGenerator|GetStream)))
        (Rendering|Material|SetVectorParameterValueonMaterials (Variables|Default|GetSK_Flag) "Flag Color" (Math|Conversions|ToVector(LinearColor) (Variables|Main|GetFlag%20Color)))
        (Rendering|Material|SetVectorParameterValueonMaterials (Variables|Default|GetSK_Flag) "Flag Border Tint" (Math|Conversions|ToVector(LinearColor) (Variables|0-Pattern|GetFlag%20Border%20Tint)))
        (Rendering|Material|SetScalarParameterValueonMaterials (Variables|Default|GetSK_Flag) "Roughness from Color" (Variables|Main|GetRoughnessFromColor))
        (CallFunction|SetNormal))
      (:then_5
        ;[1 1 1] Dirt and Gradient
        (bind _returnvalue_19 (CallFunction|RandomEnum (|GetNumEnumEntries) (Variables|RandomGenerator|GetStream)))
        (Variables|5-Dirt&Gradient|SetE_Dirt_Masks (Utilities|Enum|ByteToEnumE_Dirt_Masks _returnvalue_19))
        (Variables|5-Dirt&Gradient|SetDirt%20Power (Math|Random|RandomFloatinRangefromStream 0.03 0.07 (Variables|RandomGenerator|GetStream)))
        (Variables|5-Dirt&Gradient|SetGradient%20Bot (Utilities|Struct|MakeLinearColor (.x _returnvalue_2) (.y _returnvalue_2) (.z _returnvalue_2) (Math|Random|RandomFloatinRangefromStream 0.0 1.0 _stream_7)))
        (Variables|5-Dirt&Gradient|SetGradient%20Top (Utilities|Struct|MakeLinearColor (.x _returnvalue_7) (.y _returnvalue_7) (.z _returnvalue_7) (Math|Random|RandomFloatinRangefromStream 0.0 1.0 _stream_5)))
        (Rendering|Material|SetVectorParameterValueonMaterials (Variables|Default|GetSK_Flag) "Gradient Bot" (Math|Conversions|ToVector(LinearColor) (Variables|5-Dirt&Gradient|GetGradient%20Bot)))
        (Rendering|Material|SetVectorParameterValueonMaterials (Variables|Default|GetSK_Flag) "Gradient Top" (Math|Conversions|ToVector(LinearColor) (Variables|5-Dirt&Gradient|GetGradient%20Top)))
        (CallFunction|SetDirtMasks)
        (return)))))

(fn NextFlag
  (if (Variables|RandomGenerator|GetuseRandomGenerator?)
    (bind _result (Math|Integer|IncrementInt (Variables|RandomGenerator|GetNew%20Seed))
      (:%20%20
        (Math|Random|SetRandomStreamSeed (Variables|RandomGenerator|GetStream) _result)
        (RandomGenerator|Randomize)
        (return)))))

(fn PreviousFlag
  (if (Variables|RandomGenerator|GetuseRandomGenerator?)
    (bind _result (Math|Integer|DecrementInt (Variables|RandomGenerator|GetNew%20Seed))
      (:%20%20
        (Math|Random|SetRandomStreamSeed (Variables|RandomGenerator|GetStream) _result)
        (RandomGenerator|Randomize)
        (return)))))